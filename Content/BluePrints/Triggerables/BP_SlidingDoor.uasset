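; BP_SlidingDoor is a triggerable two-panel sliding door that opens and closes on Overlapped and UnOverlapped events.
; Overlapped plays the DoorOpenAmount timeline, which lerps the left and right door meshes from their relative origin to their respective open positions.
; UnOverlapped reverses the same timeline to slide both panels closed.
; It has no active overlap detection or Tick logic of its own.
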(event EventBeginPlay
  (|CallParentFunction) ; This node is disabled and will not be called.\nDrag off pins to build functionality.
)

(event Collision|EventActorBeginOverlap
  (params (OtherActor :type Actor%20Object%20Reference))
  (|CallParentFunction OtherActor) ; This node is disabled and will not be called.\nDrag off pins to build functionality.
)

(event EventTick
  (params (DeltaSeconds :type Float%20%28single-precision%29))
  (|CallParentFunction DeltaSeconds) ; This node is disabled and will not be called.\nDrag off pins to build functionality.
)

(event EventOverlapped
  (params (Other%20Actors :type Actor%20Object%20Reference))
  (bind _dooropenamount (Timeline|DoorOpenAmount Play)
    (:Update
      (Transformation|SetRelativeLocation (Variables|Default|GetSM_DoorLeft) (Math|Vector|Lerp(Vector) "0, 0, 0" (Variables|Default|GetL_DoorOpenPos) _dooropenamount) false false)
      (Transformation|SetRelativeLocation (Variables|Default|GetSM_DoorRight) (Math|Vector|Lerp(Vector) "0, 0, 0" (Variables|Default|GetR_DoorOpenPos) _dooropenamount) false false))))

(event EventUnOverlapped
  (params (Other%20Actors :type Actor%20Object%20Reference))
  (bind _dooropenamount (Timeline|DoorOpenAmount Reverse)
    (:Update
      (Transformation|SetRelativeLocation (Variables|Default|GetSM_DoorLeft) (Math|Vector|Lerp(Vector) "0, 0, 0" (Variables|Default|GetL_DoorOpenPos) _dooropenamount) false false)
      (Transformation|SetRelativeLocation (Variables|Default|GetSM_DoorRight) (Math|Vector|Lerp(Vector) "0, 0, 0" (Variables|Default|GetR_DoorOpenPos) _dooropenamount) false false))))

(fn ConstructionScript
  (|CallParentFunction))